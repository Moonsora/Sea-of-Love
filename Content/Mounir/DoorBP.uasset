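; DoorBP is a door actor that swings open and closed around a DoorPivot component, with sound effects.
; OpenDoor plays a bedroom door sound and runs a timeline that sets the pivot's yaw; CloseDoor reverses that timeline.
; DoorLocked plays a locked-door cue when Open is true, but OpenDoor's branch is fixed to true, so it never calls DoorLocked.
; Both sounds play at the world origin.
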(event `DoorLocked`
  (if (`self.Open`)
    (`GameplayStatics.PlaySoundAtLocation` "/Game/Emma/SFX/LockedDoor_SFX_Cue.LockedDoor_SFX_Cue" (0.0 0.0 0.0) (struct) 1.0 1.0 0.0 null null null null)))

(event `Open Door`
  (if true
    (`|ExecutionSequence`
      (:`then_0`
        (`GameplayStatics.PlaySoundAtLocation` "/Game/Emma/SFX/BedroomDoorOpen_SFX.BedroomDoorOpen_SFX" (0.0 0.0 0.0) (struct) 1.0 1.0 0.0 null null null null))
      (:`then_1`
        (bind (_direction _slideanim) (`Timeline|Timeline_0` :!label _label)
          (:`Update`
            (`SceneComponent.K2_SetRelativeRotation` (`self.Door Pivot`) (`KismetMathLibrary.MakeRotator` 0.0 0.0 _slideanim) false false)))))
    (else
      (`self.DoorLocked`))))

(event `Close Door`
  (goto _label :!via `Reverse`))

(fn `UserConstructionScript`)