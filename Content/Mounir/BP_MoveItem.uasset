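; BP_MoveItem is an interactable item actor that toggles a custom depth render when the player is nearby, likely as a highlight.
; Its construction script applies the ItemModel mesh, and Tick checks player distance against a fixed threshold to switch custom depth.
; InteractItem prints a debug "Inspect" message and returns ItemModel to the caller.
; A separate Inspect function disables the Player's input and calls EnableInput on the player controller.
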(event `self.ReceiveTick`
  (params (DeltaSeconds :type "Float (single-precision)"))
  (bind _staticmesh (`self.StaticMesh`))
  (`|ExecutionSequence`
    (:`then_0`
      (`/Engine/EditorBlueprintResources/StandardMacros.CompareFloat` (`self.GetDistanceTo` (`GameplayStatics.GetPlayerCharacter` 0)) 200.0
        (:`>`
          (`PrimitiveComponent.SetRenderCustomDepth` _staticmesh false))
        (:`<`
          (`PrimitiveComponent.SetRenderCustomDepth` _staticmesh true))))))

(fn `Inspect`
  (bind _returnvalue (`GameplayStatics.GetPlayerController` 0))
  (`self.DisableInput` (`self.Player`) _returnvalue)
  (`self.EnableInput` _returnvalue null))

(fn `InteractItem`
  (returns (ItemModel :type "StaticMesh Object Reference"))
  (`KismetSystemLibrary.PrintString` " Inspect")
  (return (`self.Item Model`)))

(fn `UserConstructionScript`
  (`StaticMeshComponent.SetStaticMesh` (`self.StaticMesh`) (`self.Item Model`)))