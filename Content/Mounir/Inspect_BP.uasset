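; Inspectable item Blueprint that shows a configurable mesh and exposes functions for interacting with it and inspecting it.
; The construction script applies ItemModel to the StaticMesh component, and InteractItem prints a debug string and returns that same model to its caller.
; Inspect disables input on the player and calls EnableInput with the player controller, but nothing in this Blueprint calls it and the event graph is empty.
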(fn `Inspect`
  (bind _returnvalue (`GameplayStatics.GetPlayerController` 0))
  (`self.DisableInput` (`self.Player`) _returnvalue)
  (`self.EnableInput` _returnvalue null))

(fn `InteractItem`
  (returns (ItemModel :type "StaticMesh Object Reference"))
  (`KismetSystemLibrary.PrintString` " Inspect")
  (return (`self.Item Model`)))

(fn `UserConstructionScript`
  (`StaticMeshComponent.SetStaticMesh` (`self.StaticMesh`) (`self.Item Model`)))