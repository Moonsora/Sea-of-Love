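; BP_Desk is a desk with a sliding drawer that gives key-pickup feedback when first opened.
; While the Vase condition is true, Tick toggles custom depth on the drawer by player proximity.
; OpenDrawer and CloseDrawer play sounds and slide the Grab component along local Y using timeline-driven lerps from its current position.
; After a delay, a DoOnce in OpenDrawer shows the key-gotten widget with a sound.
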(event `self.ReceiveTick`
  (params (DeltaSeconds :type "Float (single-precision)"))
  (bind _drawer (`self.Drawer`))
  (if (`self.Vase`)
    (`/Engine/EditorBlueprintResources/StandardMacros.CompareFloat` (`self.GetDistanceTo` (`GameplayStatics.GetPlayerCharacter` 0)) 100.0
      (:`>`
        (`PrimitiveComponent.SetRenderCustomDepth` _drawer false))
      (:`<`
        (`PrimitiveComponent.SetRenderCustomDepth` _drawer true)))))

(event `OpenDrawer`
  (bind (_relativelocation_x _relativelocation_y _relativelocation_z) (`KismetMathLibrary.BreakVector` (`SceneComponent.RelativeLocation` (`self.Grab`))))
  (`|ExecutionSequence`
    (:`then_0`
      (`GameplayStatics.PlaySoundAtLocation` "/Game/Emma/SFX/DrawerOpen_SFX_Cue.DrawerOpen_SFX_Cue" (0.0 0.0 0.0) (struct) 1.0 1.0 0.0 null null null null))
    (:`then_1`
      (set `self.Start Location` (`KismetMathLibrary.MakeVector` _relativelocation_x _relativelocation_y _relativelocation_z))
      (set `self.End Location` (`KismetMathLibrary.MakeVector` _relativelocation_x (+ _relativelocation_y 50.0) _relativelocation_z))
      (bind (_direction _newtrack_0) (`Timeline|Timeline_0` :!via `PlayFromStart`)
        (:`Update`
          (`SceneComponent.K2_SetRelativeLocation` (`self.Grab`) (`KismetMathLibrary.VLerp` (`self.Start Location`) (`self.End Location`) _newtrack_0) false false))))
    (:`then_2`
      (`KismetSystemLibrary.Delay` 2.0)
      (`/Engine/EditorBlueprintResources/StandardMacros.DoOnce` false
        (:`Completed`
          (`|ExecutionSequence`
            (:`then_0`
              (bind _returnvalue (`|CreateWidget` "/Game/Emma/UI_Assets/BPs/KeyGotten_WB.KeyGotten_WB_C"))
              (`UserWidget.AddToViewport` _returnvalue 0))
            (:`then_1`
              (`GameplayStatics.PlaySound2D` "/Game/Emma/SFX/KeyGotten_SFX_Cue.KeyGotten_SFX_Cue" 1.0 1.0 0.0 null null))))))))

(event `Close Drawer`
  (bind (_relativelocation_x _relativelocation_y _relativelocation_z) (`KismetMathLibrary.BreakVector` (`SceneComponent.RelativeLocation` (`self.Grab`))))
  (`|ExecutionSequence`
    (:`then_0`
      (`GameplayStatics.PlaySoundAtLocation` "/Game/Emma/SFX/CloseDrawer_SFX.CloseDrawer_SFX" (0.0 0.0 0.0) (struct) 1.0 1.0 0.0 null null null null))
    (:`then_1`
      (set `self.Start Location` (`KismetMathLibrary.MakeVector` _relativelocation_x _relativelocation_y _relativelocation_z))
      (set `self.End Location` (`KismetMathLibrary.MakeVector` _relativelocation_x (- _relativelocation_y 50.0) _relativelocation_z))
      (bind (_direction _newtrack_0) (`Timeline|Timeline_1` :!via `PlayFromStart`)
        (:`Update`
          (`SceneComponent.K2_SetRelativeLocation` (`self.Grab`) (`KismetMathLibrary.VLerp` (`self.Start Location`) (`self.End Location`) _newtrack_0) false false))))))

(fn `UserConstructionScript`)