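; Photo item actor that jumps to a fixed, hard-coded world position and rotation when triggered.
; The SpawbPhoto custom event runs through a DoOnce and sets the DefaultSceneRoot transform, so it moves the existing actor once and spawns nothing.
; Nothing in this Blueprint calls the event, and the other nodes are disabled defaults or unconnected leftovers.
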(event `SpawbPhoto`
  (`/Engine/EditorBlueprintResources/StandardMacros.DoOnce` false
    (:`Completed`
      (`SceneComponent.K2_SetWorldLocationAndRotation` (`self.DefaultSceneRoot`) (-172.461365 166.525772 610.809143) (struct :`Yaw` 180.0 :`Roll` -100.0) false false))))

(fn `UserConstructionScript`
  (`parent.UserConstructionScript`))