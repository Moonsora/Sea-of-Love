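; Door Blueprint for a bedroom door that opens only when its BedroomKey flag is set.
; OpenDoor plays a timeline that sets DoorPivot's yaw, plays the opening sound and removes the KeyGotten_WB widget from the screen.
; Without the key it calls DoorLocked, which plays a locked sound only if Open is true.
; CloseDoor reverses the timeline, and both sounds play at world origin rather than at the door.
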(event `DoorLocked`
  (if (`self.Open`)
    (`GameplayStatics.PlaySoundAtLocation` "/Game/Emma/SFX/LockedDoor_SFX_Cue.LockedDoor_SFX_Cue" (0.0 0.0 0.0) (struct) 1.0 1.0 0.0 null null null null)))

(event `Open Door`
  (if (`self.BedroomKey`)
    (`|ExecutionSequence`
      (:`then_0`
        (bind (_direction _slideanim) (`Timeline|Timeline_0` :!label _label)
          (:`Update`
            (`SceneComponent.K2_SetRelativeRotation` (`self.Door Pivot`) (`KismetMathLibrary.MakeRotator` 0.0 0.0 _slideanim) false false))))
      (:`then_1`
        (`GameplayStatics.PlaySoundAtLocation` "/Game/Emma/SFX/BedroomDoorOpen_SFX.BedroomDoorOpen_SFX" (0.0 0.0 0.0) (struct) 1.0 1.0 0.0 null null null null)
        (bind _foundwidgets (`WidgetBlueprintLibrary.GetAllWidgetsOfClass` "/Game/Emma/UI_Assets/BPs/KeyGotten_WB.KeyGotten_WB_C"))
        (`Widget.RemoveFromParent` (`|GetArrayItem` _foundwidgets))))
    (else
      (`self.DoorLocked`))))

(event `Close Door`
  (goto _label :!via `Reverse`))

(fn `UserConstructionScript`)