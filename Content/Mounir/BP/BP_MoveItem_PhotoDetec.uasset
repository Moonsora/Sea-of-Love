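; Actor Blueprint that rings a doorbell sound three times, five seconds apart, as a one-shot event.
; Tick calls the Ding event while the Sonette flag is true, and Ding also sets that flag after the first ring.
; A DoOnce keeps the repeated calls from restarting the sequence, and the sounds play at the world origin.
; Nothing in this graph starts the first ring or implements the item movement or photo detection suggested by the name.
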(event `self.ReceiveTick`
  (params (DeltaSeconds :type "Float (single-precision)"))
  (`parent.ReceiveTick` DeltaSeconds)
  (if (`self.Sonette`)
    (`self.Ding`)))

(event `Ding`
  (`/Engine/EditorBlueprintResources/StandardMacros.DoOnce` false
    (:`Completed`
      (`GameplayStatics.PlaySoundAtLocation` "/Game/Emma/SFX/Doorbell_Ringing.Doorbell_Ringing" (0.0 0.0 0.0) (struct) 1.0 1.0 0.0 null null null null)
      (set `self.Sonette` true)
      (`KismetSystemLibrary.Delay` 5.0)
      (`GameplayStatics.PlaySoundAtLocation` "/Game/Emma/SFX/Doorbell_Ringing.Doorbell_Ringing" (0.0 0.0 0.0) (struct) 1.0 1.0 0.0 null null null null)
      (`KismetSystemLibrary.Delay` 5.0)
      (`GameplayStatics.PlaySoundAtLocation` "/Game/Emma/SFX/Doorbell_Ringing.Doorbell_Ringing" (0.0 0.0 0.0) (struct) 1.0 1.0 0.0 null null null null))))

(fn `UserConstructionScript`
  (`parent.UserConstructionScript`))