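; Wardrobe actor that swings its left door open and closed around its yaw axis, driven by the Slide flag.
; Every Tick calls Open or Close, which play the Door timeline from start or reverse it to rotate LDoor.
; Open restarts the timeline on every frame that Slide stays true.
; A disconnected, delayed open/close sequence that also calls right-door events never runs.
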(event `self.ReceiveBeginPlay`)

(event `self.ReceiveTick`
  (params (DeltaSeconds :type "Float (single-precision)"))
  (if (`self.Slide`)
    (`self.Open`)
    (else
      (`self.Close`))))

(event `Open`
  (bind (_direction _newtrack_0) (`Timeline|Door` :!via `PlayFromStart` :!label _label)
    (:`Update`
      (`SceneComponent.K2_SetRelativeRotation` (`self.LDoor`) (`KismetMathLibrary.MakeRotator` 0.0 0.0 (* _newtrack_0 -120.0)) false false))))

(event `Close`
  (goto _label :!via `Reverse`))

(fn `UserConstructionScript`)