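; Wardrobe actor Blueprint with two hinged doors that play a timed open and close sequence on BeginPlay, with no player interaction.
; After a delay the left door opens, then it closes as the right door opens, and finally the right door closes.
; Each door has its own Timeline scaling relative yaw in opposite directions, with closing done by reversing that Timeline.
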(event `self.ReceiveBeginPlay`
  (`KismetSystemLibrary.Delay` 2.0)
  (`self.LeftDoorOpen`)
  (`KismetSystemLibrary.Delay` 2.0)
  (`self.LeftDoorClose`)
  (`self.RightDoorOpen`)
  (`KismetSystemLibrary.Delay` 2.0)
  (`self.RightDoorClose`))

(event `LeftDoorOpen`
  (bind (_direction _newtrack_0) (`Timeline|Door` :`NewTime` 0.0 :!via `PlayFromStart` :!label _label)
    (:`Update`
      (`SceneComponent.K2_SetRelativeRotation` (`self.LDoor`) (`KismetMathLibrary.MakeRotator` 0.0 0.0 (* _newtrack_0 110.0)) false false))))

(event `LeftDoorClose`
  (goto _label :!via `Reverse`))

(event `RightDoorOpen`
  (bind (_direction _newtrack_0) (`Timeline|Timeline_0` :!via `PlayFromStart` :!label _label_2)
    (:`Update`
      (`SceneComponent.K2_SetRelativeRotation` (`self.RDoor`) (`KismetMathLibrary.MakeRotator` 0.0 0.0 (* _newtrack_0 -110.0)) false false))))

(event `RightDoorClose`
  (goto _label_2 :!via `Reverse`))

(fn `UserConstructionScript`)