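; Base item actor that the player can approach and inspect, with its mesh set from ItemModel in the construction script.
; Tick checks the distance to the player character and turns on the mesh's custom depth within 200 units, off beyond.
; Inspect disables input on the Player reference, then calls EnableInput on the player controller.
; InteractItem is an empty stub.
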(event `self.ReceiveTick`
  (params (DeltaSeconds :type "Float (single-precision)"))
  (bind _mesh (`self.Mesh`))
  (`/Engine/EditorBlueprintResources/StandardMacros.CompareFloat` (`self.GetDistanceTo` (`GameplayStatics.GetPlayerCharacter` 0)) 200.0
    (:`>`
      (`PrimitiveComponent.SetRenderCustomDepth` _mesh false))
    (:`<`
      (`PrimitiveComponent.SetRenderCustomDepth` _mesh true))))

(fn `Inspect`
  (bind _returnvalue (`GameplayStatics.GetPlayerController` 0))
  (`self.DisableInput` (`self.Player`) _returnvalue)
  (`self.EnableInput` _returnvalue null))

(fn `InteractItem`
  (returns (ItemModel :type "StaticMesh Object Reference"))
  (return null))

(fn `UserConstructionScript`
  (`StaticMeshComponent.SetStaticMesh` (`self.Mesh`) (`self.ItemModel`)))